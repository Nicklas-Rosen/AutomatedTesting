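; Base pickup item Blueprint that can be highlighted, interacted with and queried as an inventory pickup.
; Highlight toggles custom depth rendering with a fixed stencil value on all primitive components, likely feeding an outline post-process.
; Interaction destroys the actor, while IsPickup returns its can-pick-up flag and item details to the caller.
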(event `/Game/LocoStarterKit/Blueprints/Interfaces/UsableInterface.Hightlight`
  (params (Active :type Boolean))
  (for _array_element (`self.K2_GetComponentsByClass` "/Script/Engine.PrimitiveComponent")
    (`PrimitiveComponent.SetRenderCustomDepth` _array_element Active)
    (`PrimitiveComponent.SetCustomDepthStencilValue` _array_element 1)))

(event `/Game/LocoStarterKit/Blueprints/Interfaces/UsableInterface.Interaction`
  (params (Interactor :type "Actor Object Reference"))
  (`self.K2_DestroyActor`))

(fn `IsPickup`
  (returns (Pickup :type Boolean) (`Inventory Item` :type "/Game/LocoStarterKit/Blueprints/Item Structure"))
  (return (`self.Can Pick up`) (`self.Item Details`)))

(fn `UserConstructionScript`
  (`parent.UserConstructionScript`))