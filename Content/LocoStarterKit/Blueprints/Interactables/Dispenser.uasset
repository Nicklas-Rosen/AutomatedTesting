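; Interactable dispenser that spawns a configurable item when the interactor passes a check for a required item, otherwise printing a token-needed message.
; The item spawns at SpawnPos immediately, then after a short delay a timeline swings the hinged door and slides the pusher from its cached origin.
; A Busy flag blocks further use until the animation finishes.
; The construction script applies the configurable label text and color.
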(event `self.ReceiveBeginPlay`
  (set `self.PusherOrigin` (`SceneComponent.RelativeLocation` (`self.Pusher`))))

(event `/Game/LocoStarterKit/Blueprints/Interfaces/UsableInterface.Interaction`
  (params (Interactor :type "Actor Object Reference"))
  (if (not (`self.Busy`))
    (bind _hasitem (message `/Game/LocoStarterKit/Blueprints/Interfaces/HeroInterface.HasItem` Interactor (`self.Requires Item`)))
    (if _hasitem
      (set `self.Busy` true)
      (`|ExecutionSequence`
        (:`then_0`
          (`|SpawnActorFromClass` (`self.Spawns Item`) (`SceneComponent.K2_GetComponentToWorld` (`self.SpawnPos`)) "Undefined" "OverrideRootScale" null null))
        (:`then_1`
          (`KismetSystemLibrary.Delay` 2.0)
          (bind (_direction _door _pusher) (`Timeline|DispenerAnim` :!via `PlayFromStart`)
            (:`Update`
              (`SceneComponent.K2_SetRelativeRotation` (`self.Hinge`) (`KismetMathLibrary.MakeRotator` (* (* _door 45.0) -1.0)) false false)
              (`SceneComponent.K2_SetRelativeLocation` (`self.Pusher`) (+ (`self.PusherOrigin`) (`KismetMathLibrary.MakeVector` 0.0 (* _pusher (`self.PusherDistance`)))) false false))
            (:`Finished`
              (set `self.Busy` false)))))
      (else
        (`KismetSystemLibrary.PrintString` "You need a Token for this Device!")))))

(fn `UserConstructionScript`
  (bind _textrender (`self.TextRender`))
  (`parent.UserConstructionScript`)
  (`TextRenderComponent.K2_SetText` _textrender (`self.Text`))
  (`TextRenderComponent.SetTextRenderColor` _textrender (`self.TextColor`)))