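; An interactable big door that opens and closes on the Interaction event and can be locked behind a required item.
; When locked, it checks the interactor for the item, then either unlocks and toggles immediately or prints which item is needed.
; A timeline played forward or in reverse rotates the static mesh up to 90 degrees on pitch.
; The construction script applies configurable text and color to a text render label.
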(event `/Game/LocoStarterKit/Blueprints/Interfaces/UsableInterface.Interaction`
  (params (Interactor :type "Actor Object Reference"))
  (bind _requires_item (`self.Requires Item`))
  (if (`self.Locked`)
    (bind _hasitem (message `/Game/LocoStarterKit/Blueprints/Interfaces/HeroInterface.HasItem` Interactor _requires_item))
    (if _hasitem
      (`KismetSystemLibrary.PrintString` "Door has Been UNLOCKED!")
      (set `self.Locked` false)
      (bind _output_get (set `self.Open` (not (`self.Open`)) :!label _label))
      (if _output_get
        (bind (_direction _door) (`Timeline|DoorTimeline` :!label _label_2)
          (:`Update`
            (`SceneComponent.K2_SetRelativeRotation` (`self.StaticMesh`) (`KismetMathLibrary.MakeRotator` 0.0 (* (* _door 90.0) -1.0)) false false)))
        (else
          (goto _label_2 :!via `Reverse`)))
      (else
        (`KismetSystemLibrary.PrintString` (`KismetStringLibrary.Concat_StrStr` "LOCKED! Requires " (`KismetSystemLibrary.GetClassDisplayName` _requires_item) " to unlock!"))))
    (else
      (goto _label))))

(fn `UserConstructionScript`
  (bind _textrender (`self.TextRender`))
  (`parent.UserConstructionScript`)
  (`TextRenderComponent.K2_SetText` _textrender (`self.Text`))
  (`TextRenderComponent.SetTextRenderColor` _textrender (`self.TextColor`)))