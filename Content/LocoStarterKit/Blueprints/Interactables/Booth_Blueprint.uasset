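; Interactable booth with a pair of hinged doors that a player can open and close, optionally locked behind a required item.
; On Interaction, a locked booth asks the interactor for the required item, then either unlocks and toggles or prints a requirement message.
; A timeline plays forward or in reverse to swing both hinges in opposite directions up to a quarter turn.
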(event `/Game/LocoStarterKit/Blueprints/Interfaces/UsableInterface.Interaction`
  (params (Interactor :type "Actor Object Reference"))
  (bind _requires_item (`self.Requires Item`))
  (if (`self.Locked`)
    (bind _hasitem (message `/Game/LocoStarterKit/Blueprints/Interfaces/HeroInterface.HasItem` Interactor _requires_item))
    (if _hasitem
      (set `self.Locked` false)
      (bind _output_get (set `self.Open` (not (`self.Open`)) :!label _label))
      (if _output_get
        (bind (_direction _door) (`Timeline|DoorTimeline` :!label _label_2)
          (:`Update`
            (bind _returnvalue (* _door 90.0))
            (`SceneComponent.K2_SetRelativeRotation` (`self.Hinge`) (`KismetMathLibrary.MakeRotator` 0.0 0.0 _returnvalue) false false)
            (`SceneComponent.K2_SetRelativeRotation` (`self.Hinge1`) (`KismetMathLibrary.MakeRotator` 0.0 0.0 (* _returnvalue -1.0)) false false)))
        (else
          (goto _label_2 :!via `Reverse`)))
      (else
        (`KismetSystemLibrary.PrintString` (`KismetStringLibrary.Concat_StrStr` "Requires " (`KismetSystemLibrary.GetClassDisplayName` _requires_item) " to Unlock"))))
    (else
      (goto _label))))

(fn `UserConstructionScript`
  (`parent.UserConstructionScript`))