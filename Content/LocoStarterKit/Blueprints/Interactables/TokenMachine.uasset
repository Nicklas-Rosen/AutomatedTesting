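; Interactable token machine that stays unfixed until the player interacts while holding the required item, then spawns Tokens.
; A timeline spins one gear from BeginPlay, adds the others once fixed, and its event track spawns Tokens while the box holds fewer than the limit.
; Interacting with the item fixes it and shows the missing gear, unless Malfunctioning, when it launches a MachinePart instead.
; Custom depth stencil highlights the unfixed machine.
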(event `self.ReceiveBeginPlay`
  (set `self.Gear1BaseRot` (`SceneComponent.RelativeRotation` (`self.Gear1`)))
  (set `self.Gear2BaseRot` (`SceneComponent.RelativeRotation` (`self.Gear2`)))
  (bind (_direction _gears) (`Timeline|Timeline_0` :!via `PlayFromStart`)
    (:`Update`
      (bind _returnvalue (* _gears 360.0))
      (`SceneComponent.K2_SetRelativeRotation` (`self.Gear1`) (`KismetMathLibrary.ComposeRotators` (`self.Gear1BaseRot`) (`KismetMathLibrary.MakeRotator` 0.0 _returnvalue)) false false)
      (if (`self.Fixed`)
        (`SceneComponent.K2_SetRelativeRotation` (`self.Gear2`) (`KismetMathLibrary.ComposeRotators` (`self.Gear2BaseRot`) (`KismetMathLibrary.MakeRotator` 0.0 _returnvalue)) false false)
        (`SceneComponent.K2_SetRelativeRotation` (`self.MissingGear`) (`KismetMathLibrary.MakeRotator` 0.0 0.0 _returnvalue) false false)))
    (:`Spawner`
      (if (and (< (`KismetArrayLibrary.Array_Length` (`PrimitiveComponent.GetOverlappingActors` (`self.Box`) "/Game/LocoStarterKit/Blueprints/Items/Token.Token_C")) (`self.TokenLimit`)) (`self.Fixed`))
        (`|SpawnActorFromClass` "/Game/LocoStarterKit/Blueprints/Items/Token.Token_C" (`SceneComponent.K2_GetComponentToWorld` (`self.Spawner`)) "AdjustIfPossibleButAlwaysSpawn" "OverrideRootScale" null null)))))

(event `/Game/LocoStarterKit/Blueprints/Interfaces/UsableInterface.Hightlight`
  (params (Active :type Boolean))
  (bind _gear2 (`self.Gear2`))
  (if (not (`self.Fixed`))
    (`PrimitiveComponent.SetRenderCustomDepth` _gear2 Active)
    (`PrimitiveComponent.SetRenderCustomDepth` (`self.Gear1`) Active)
    (`PrimitiveComponent.SetRenderCustomDepth` (`self.Cylinder`) Active)
    (`PrimitiveComponent.SetCustomDepthStencilValue` _gear2 1)
    (`PrimitiveComponent.SetCustomDepthStencilValue` (`self.Gear1`) 1)
    (`PrimitiveComponent.SetCustomDepthStencilValue` (`self.Cylinder`) 1)))

(event `/Game/LocoStarterKit/Blueprints/Interfaces/UsableInterface.Interaction`
  (params (Interactor :type "Actor Object Reference"))
  (bind _returnvalue (`SceneComponent.K2_GetComponentToWorld` (`self.GearSpit`)))
  (if (not (`self.Fixed`))
    (bind _hasitem (message `/Game/LocoStarterKit/Blueprints/Interfaces/HeroInterface.HasItem` Interactor (`self.Requires Item`)))
    (if _hasitem
      (if (`self.Malfunctioning`)
        (bind _returnvalue_2 (`|SpawnActorFromClass` "/Game/LocoStarterKit/Blueprints/Items/MachinePart.MachinePart_C" _returnvalue "AdjustIfPossibleButAlwaysSpawn" "OverrideRootScale" null null))
        (`PrimitiveComponent.AddImpulseAtLocation` (`/Game/LocoStarterKit/Blueprints/Items/PickupBase.StaticMesh` _returnvalue_2) (* (`KismetMathLibrary.GetUpVector` (.rotation _returnvalue)) 10000.0) (.location _returnvalue) "None")
        (else
          (set `self.Fixed` true)
          (`SceneComponent.SetVisibility` (`self.MissingGear`) true false)
          (`PrimitiveComponent.SetRenderCustomDepth` (`self.Gear2`) false)
          (`PrimitiveComponent.SetRenderCustomDepth` (`self.Gear1`) false)
          (`PrimitiveComponent.SetRenderCustomDepth` (`self.Cylinder`) false)))
      (else
        (`KismetSystemLibrary.PrintString` "This Machine Is missing something...")))))

(fn `UserConstructionScript`
  (`parent.UserConstructionScript`)
  (`SceneComponent.SetVisibility` (`self.MissingGear`) (`self.Broken`) false))